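; BP_RobotArm is an industrial robot arm whose end control follows a scene component through Control Rig.
; BeginPlay maps the skeletal mesh to the Control Rig as output, stores PointScene as Point, moves it to the Default transform's location and sets a move speed.
; Each Tick writes PointScene's world location to the end control, so moving that component poses the arm.
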(event EventBeginPlay
  (Variables|Default|SetPoint (Variables|Default|GetPointScene))
  (Class|ControlRigComponent|AddMappedCompleteSkeletalMesh (Variables|Default|GetControlRig) (Variables|Default|GetSK_IndustrialRobot) "Output")
  (Transformation|SetRelativeLocation (Variables|Default|GetPointScene) (.location (Transformation|GetRelativeTransform (Variables|Default|GetDefault))) false false)
  (Variables|Default|SetMoveSpeed 3e+02))

(event EventTick
  (params (DeltaSeconds :type Float%20%28single-precision%29))
  (Class|ControlRigComponent|SetControlTransform (Variables|Default|GetControlRig) "Robot1_End_Control" (Math|Transform|MakeTransform (Transformation|GetWorldLocation (Variables|Default|GetPointScene)) "0, 0, 0" "1.000000,1.000000,1.000000") "WorldSpace"))

(fn ConstructionScript)