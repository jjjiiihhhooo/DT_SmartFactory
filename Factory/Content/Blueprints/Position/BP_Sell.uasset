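; BP_Sell is a position actor that hosts a pair of robot arms and a state indicator cube.
; On BeginPlay it spawns BP_RightRobotArm and BP_LeftRobotArm at their spawn component transforms, storing each and passing itself as ParentSell.
; StateCubeChange swaps the cube's material, applying the default material when Active is true and the active material when false.
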(event EventBeginPlay
  (Utilities|FlowControl|Sequence
    (:then_0
      (bind _returnvalue (Game|SpawnActorfromClass "/Game/Blueprints/Robot/BP_RightRobotArm.BP_RightRobotArm_C" (Transformation|GetWorldTransform (Variables|Default|GetRightRobotArmSpawn)) "Undefined" "MultiplyWithRoot" 0 0))
      (bind _output_get (Variables|Default|SetRightRobotArm _returnvalue))
      (Variables|/Script/Factory.RobotArm|SetParentSell _output_get self))
    (:then_1
      (bind _returnvalue_2 (Game|SpawnActorfromClass "/Game/Blueprints/Robot/BP_LeftRobotArm.BP_LeftRobotArm_C" (Transformation|GetWorldTransform (Variables|Default|GetLeftRobotArmSpawn)) "Undefined" "MultiplyWithRoot" 0 0))
      (bind _output_get_2 (Variables|Default|SetLeftRobotArm _returnvalue_2))
      (Variables|/Script/Factory.RobotArm|SetParentSell _output_get_2 self))))

(fn ConstructionScript)

(fn StateCubeChange
  (params (Active :type Boolean))
  (if Active
    (Rendering|Material|SetMaterial (Variables|Default|GetSellStateCube) 0 "/Game/Materials/MyMat/SellStateDefaultMat.SellStateDefaultMat")
    (else
      (Rendering|Material|SetMaterial (Variables|Default|GetSellStateCube) 0 "/Game/Materials/MyMat/SellStateActiveMat.SellStateActiveMat"))))